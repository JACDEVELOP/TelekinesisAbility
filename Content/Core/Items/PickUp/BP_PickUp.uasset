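; BP_PickUp is an interactable pickup actor that characters can pick up, with its mesh and interaction animation driven by a data asset.
; The construction script applies the data asset's static mesh.
; On Interact, it casts the actor to LT_CharacterBase, sets it as the PickUpComponent's holder, plays the montage and triggers the pickup.
; It then registers itself as the current PickUp on that actor's LT_InventoryComponent, if present.
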(event EventBeginPlay)

(event Collision|EventActorBeginOverlap
  (params (OtherActor :type Actor%20Object%20Reference)))

(event EventTick
  (params (DeltaSeconds :type Float%20%28single-precision%29)))

(event EventInteract
  (params (InteractActor :type Actor%20Object%20Reference))
  (bind _returnvalue (Actor|GetComponentbyClass InteractActor "/Script/LiquidTest.LT_InventoryComponent"))
  (bind _pickupcomponent (Variables|Default|GetPickUpComponent))
  (bind _aslt_character_base (Utilities|Casting|CastToLT_CharacterBase InteractActor))
  (Variables|/Script/LiquidTest.LT_PickUpComponent|SetHolder _pickupcomponent _aslt_character_base)
  (Animation|PlayAnimMontage _aslt_character_base (Variables|/Script/LiquidTest.LT_ActorInteractuableDataAsset|GetInteractAnimation (Variables|Default|GetDataAsset)) 1.0 "None")
  (Class|LTPickUpComponent|PickUpObject _pickupcomponent)
  (Utilities|IsValid _returnvalue
    (:Is%20Valid
      (Variables|/Script/LiquidTest.LT_InventoryComponent|SetPickUp _returnvalue self))))

(fn ConstructionScript
  (Components|StaticMesh|SetStaticMesh (Variables|Default|GetStaticMesh) (Variables|/Script/LiquidTest.LT_ActorInteractuableDataAsset|GetStaticMesh (Variables|Default|GetDataAsset))))